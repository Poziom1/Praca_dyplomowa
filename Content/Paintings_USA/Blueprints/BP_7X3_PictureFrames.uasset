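; Wall picture Blueprint that shows a painting as one 7X3 frame or split across two or three panels, in three selectable frame styles.
; The construction script adds a mesh per panel, chosen by count, position and style, and offsets multiple panels along local Y by Spacing plus a style-specific width.
; Split panels share one dynamic instance of PictureMaterial with a count-specific canvas mask texture, while a single frame uses the material directly.
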(fn `UserConstructionScript`
  (bind _returnvalue (+ (`self.Spacing`) (select `int` (- (`self.Frame type`) 1) :`0` 111.25 :`1` 103.5 :`2` 103.5)))
  (bind _returnvalue_2 (+ (`self.Spacing`) (select `int` (- (`self.Frame type`) 1) :`0` 68.25 :`1` 64.25 :`2` 64.25)))
  (if (> (`self.Number of picture frames`) 1)
    (bind _returnvalue_3 (`KismetMaterialLibrary.CreateDynamicMaterialInstance` (`self.Picture material`)))
    (for _index (range 1 (+ (`self.Number of picture frames`) 1))
      (bind _returnvalue_4 (- _index 1))
      (bind _returnvalue_5 (`AddComponent|NODE_AddStaticMeshComponent-1` :`RelativeTransform` (`KismetMathLibrary.MakeTransform` (`KismetMathLibrary.MakeVector` 0.0 (`KismetMathLibrary.SelectFloat` (select `int` _returnvalue_4 :`0` _returnvalue_2 :`1` (* _returnvalue_2 -1.0)) (select `int` _returnvalue_4 :`0` _returnvalue :`1` 0.0 :`2` (* _returnvalue -1.0)) (== (`self.Number of picture frames`) 2))))))
      (`StaticMeshComponent.SetStaticMesh` _returnvalue_5 (select `int` (- (`self.Number of picture frames`) 2) :`0` (select `int` _returnvalue_4 :`0` (select `int` (- (`self.Frame type`) 1) :`0` "/Game/Paintings_USA/Geometry/SM_PictureFrame_4X4-1A.SM_PictureFrame_4X4-1A" :`1` "/Game/Paintings_USA/Geometry/SM_PictureFrame_4X4-2A.SM_PictureFrame_4X4-2A" :`2` "/Game/Paintings_USA/Geometry/SM_PictureFrame_4X4-3A.SM_PictureFrame_4X4-3A" :!type "StaticMesh Object Reference") :`1` (select `int` (- (`self.Frame type`) 1) :`0` "/Game/Paintings_USA/Geometry/SM_PictureFrame_4X4-1B.SM_PictureFrame_4X4-1B" :`1` "/Game/Paintings_USA/Geometry/SM_PictureFrame_4X4-2B.SM_PictureFrame_4X4-2B" :`2` "/Game/Paintings_USA/Geometry/SM_PictureFrame_4X4-3B.SM_PictureFrame_4X4-3B" :!type "StaticMesh Object Reference")) :`1` (select `int` _returnvalue_4 :`0` (select `int` (- (`self.Frame type`) 1) :`0` "/Game/Paintings_USA/Geometry/SM_PictureFrame_3X4-1A.SM_PictureFrame_3X4-1A" :`1` "/Game/Paintings_USA/Geometry/SM_PictureFrame_3X4-2A.SM_PictureFrame_3X4-2A" :`2` "/Game/Paintings_USA/Geometry/SM_PictureFrame_3X4-3A.SM_PictureFrame_3X4-3A" :!type "StaticMesh Object Reference") :`1` (select `int` (- (`self.Frame type`) 1) :`0` "/Game/Paintings_USA/Geometry/SM_PictureFrame_3X4-1B.SM_PictureFrame_3X4-1B" :`1` "/Game/Paintings_USA/Geometry/SM_PictureFrame_3X4-2B.SM_PictureFrame_3X4-2B" :`2` "/Game/Paintings_USA/Geometry/SM_PictureFrame_3X4-3B.SM_PictureFrame_3X4-3B" :!type "StaticMesh Object Reference") :`2` (select `int` (- (`self.Frame type`) 1) :`0` "/Game/Paintings_USA/Geometry/SM_PictureFrame_3X4-1C.SM_PictureFrame_3X4-1C" :`1` "/Game/Paintings_USA/Geometry/SM_PictureFrame_3X4-2C.SM_PictureFrame_3X4-2C" :`2` "/Game/Paintings_USA/Geometry/SM_PictureFrame_3X4-3C.SM_PictureFrame_3X4-3C" :!type "StaticMesh Object Reference"))))
      (`PrimitiveComponent.SetMaterial` _returnvalue_5 (`self.Picture Material index`) _returnvalue_3)
      (`MaterialInstanceDynamic.SetTextureParameterValue` _returnvalue_3 "Diffuse Texture Mask" (select `int` (- (`self.Number of picture frames`) 2) :`0` "/Game/Paintings_USA/Textures/Shared/T_CanvasMask2.T_CanvasMask2" :`1` "/Game/Paintings_USA/Textures/Shared/T_CanvasMask3.T_CanvasMask3" :!type "Texture Object Reference")))
    (else
      ;[1 1 1] Setup single frame
      (bind _returnvalue_6 (`AddComponent|NODE_AddStaticMeshComponent-0`))
      (`StaticMeshComponent.SetStaticMesh` _returnvalue_6 (select `int` (- (`self.Frame type`) 1) :`0` "/Game/Paintings_USA/Geometry/SM_PictureFrame_7X3-1.SM_PictureFrame_7X3-1" :`1` "/Game/Paintings_USA/Geometry/SM_PictureFrame_7X3-2.SM_PictureFrame_7X3-2" :`2` "/Game/Paintings_USA/Geometry/SM_PictureFrame_7X3-3.SM_PictureFrame_7X3-3" :!type "StaticMesh Object Reference"))
      (`PrimitiveComponent.SetMaterial` _returnvalue_6 (`self.Picture Material index`) (`self.Picture material`)))))